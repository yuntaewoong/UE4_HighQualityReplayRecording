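; Player controller for replay playback in a path tracing recording game, handling replay restart, customization and saving of the video capture.
; Custom events restart and pause the replay, or apply game-instance replay info (fixed framerate and character mesh) before toggling demopause.
; On the remote Tick branch, a replay ending during capture saves the video and opens the capture result UI with mouse input.
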(event Custom|ResetReplayToTime0
  (Class|ReplayPlayerController|RestartReplay)
  (Utilities|FlowControl|Delay 0.1)
  (Development|ExecuteConsoleCommand "demopause" 0)
  (Development|PrintString "Replay Setting And Pause"))

(event Custom|RestartWithCustom
  (bind _aspath_tracing_record_game_instance_bp (Utilities|Casting|CastToPathTracingRecordGameInstanceBP (Game|GetGameInstance)))
  (bind _newparam (Default|GetReplayInfo _aspath_tracing_record_game_instance_bp))
  (CallFunction|Customize _newparam)
  (Development|ExecuteConsoleCommand "demopause" 0))

(event EventTick
  (params (DeltaSeconds :type Float%20%28single-precision%29))
  (bind _returnvalue (Game|GetPlayerController 0))
  (Networking|SwitchHasAuthority
    (:Remote
      (bind _returnvalue_2 (Class|ReplayPlayerController|IsReplayEnd))
      (if (and _returnvalue_2 (Variables|Default|GetIsCapturing))
        (Class|SimpleVideoCaptureSubsystem|SaveVideoCapture (Subsystems|GetSimpleVideoCaptureSubsystem))
        (Development|PrintString "Save Replay")
        (Variables|Default|SetIsCapturing false)
        (bind _returnvalue_3 (UserInterface|CreateWidget "/Game/Manager/CaptureResultUI.CaptureResultUI_C"))
        (UserInterface|Viewport|AddtoViewport _returnvalue_3 0)
        (Input|SetInputModeUIOnly _returnvalue 0 "DoNotLock")
        (Variables|/Script/Engine.PlayerController|SetbShowMouseCursor _returnvalue true)))))

(fn ConstructionScript)

(fn Customize
  (params (CustomizingInfo :type Replay%20Custom%20Structure))
  (bind (_replayfilename _replayresolution _replayframerate _replaycharacter) (Utilities|Struct|BreakReplayCustom CustomizingInfo))
  (Utilities|FlowControl|Sequence
    (:then_0
      (bind _aspath_tracing_recording_game_instance (Utilities|Casting|CastToPathTracingRecordingGameInstance (Game|GetGameInstance)))
      (Class|PathTracingRecordingGameInstance|SetBUseFixedFramerate _aspath_tracing_recording_game_instance true)
      (Class|PathTracingRecordingGameInstance|SetFixedFramerate _aspath_tracing_recording_game_instance _replayframerate))
    (:then_1
      (bind _returnvalue (Actor|GetActorOfClass "/Game/Player/PathTracingRecordCharacterBP.PathTracingRecordCharacterBP_C"))
      (Development|PrintString "HelloPlayer")
      (switch string _replaycharacter
        (:FrostGiant
          (Class|SkinnedMeshComponent|SetSkeletalMesh (Variables|/Script/Engine.Character|GetMesh _returnvalue) "/Game/InfinityBladeWarriors/Character/CompleteCharacters/SK_CharM_FrostGiant.SK_CharM_FrostGiant" true))
        (:CardBoard
          (Class|SkinnedMeshComponent|SetSkeletalMesh (Variables|/Script/Engine.Character|GetMesh _returnvalue) "/Game/InfinityBladeWarriors/Character/CompleteCharacters/SK_CharM_Cardboard.SK_CharM_Cardboard" true))
        (:Robo
          (Class|SkinnedMeshComponent|SetSkeletalMesh (Variables|/Script/Engine.Character|GetMesh _returnvalue) "/Game/InfinityBladeWarriors/Character/CompleteCharacters/SK_CharM_Robo.SK_CharM_Robo" true))))))