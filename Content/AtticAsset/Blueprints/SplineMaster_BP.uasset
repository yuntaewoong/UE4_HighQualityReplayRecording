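; SplineMaster_BP is a spline mesh actor that lays a chosen static mesh along an editable spline.
; Its construction script adds one spline mesh component per segment between consecutive points, using the set mesh and forward axis.
; Each component attaches to the spline and bends to the local positions and tangents of its two endpoints, with collision disabled.
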(fn ConstructionScript
  (bind _spline (Variables|Default|GetSpline))
  (for _index (range 0 (- (Spline|GetNumberOfSplinePoints _spline) 2))
    (bind _returnvalue (AddComponent|AddSplineMeshComponent false))
    (Components|StaticMesh|SetStaticMesh _returnvalue (Variables|Default|Getmesh))
    (SplineMesh|SetForwardAxis _returnvalue (Variables|Default|Getforwardaxis) true)
    (Collision|SetCollisionEnabled _returnvalue "NoCollision")
    (Transformation|AttachComponentToComponent _returnvalue _spline "None" "KeepRelative" "KeepRelative" "KeepRelative" true)
    (SplineMesh|SetStartandEnd _returnvalue (Spline|GetLocationatSplinePoint _spline _index "Local") (Spline|GetTangentatSplinePoint _spline _index "Local") (Spline|GetLocationatSplinePoint _spline (+ _index 1) "Local") (Spline|GetTangentatSplinePoint _spline (+ _index 1) "Local") true :!class /Script/Engine.SplineMeshComponent)))