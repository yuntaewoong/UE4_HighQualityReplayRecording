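; Manager Blueprint that starts and stops named replay recordings from player input.
; The start action opens RecordNameSettingUI with a back-reference and UI-only input, setting the recording flag immediately, before recording begins.
; StartRecording removes the widget, passes the file name to PathTracingRecordingGameInstance and restores game-and-UI input with a hidden cursor.
; StopRecording forwards to the game instance and clears the flag; ReplayRecording is an empty stub.
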(event EventBeginPlay
  (Input|EnableInput (Game|GetPlayerController 0)))

(event Input|ActionEvents|InputActionStartRecording
  (params (Key :type Key%20Structure :default "None"))
  (bind _returnvalue (Game|GetPlayerController 0))
  ;[1 1 1] Recording시작
  (:Pressed
    (bind _returnvalue_2 (Class|RecordingManager|GetIsRecording))
    (if (not _returnvalue_2)
      (bind _returnvalue_3 (UserInterface|CreateWidget "/Game/Manager/RecordNameSettingUI.RecordNameSettingUI_C"))
      (bind _output_get (Variables|Default|SetRecordNameSettingUI _returnvalue_3))
      (Variables|/Game/Manager/RecordNameSettingUI.RecordNameSettingUI_C|SetRecordingManagerBP _output_get self)
      (UserInterface|Viewport|AddtoViewport (Variables|Default|GetRecordNameSettingUI) 0)
      (Input|SetInputModeUIOnly _returnvalue (Variables|Default|GetRecordNameSettingUI) "DoNotLock")
      (Variables|/Script/Engine.PlayerController|SetbShowMouseCursor _returnvalue true)
      (Class|RecordingManager|SetIsRecording true))))

(event Input|ActionEvents|InputActionStopRecording
  (params (Key :type Key%20Structure :default "None"))
  ;[1 1 1] Recording종료
  (:Pressed
    (CallFunction|StopRecording)))

(event Input|ActionEvents|InputActionReplayRecording
  (params (Key :type Key%20Structure :default "None")))

(fn ConstructionScript)

(fn StartRecording
  (params (ReplayFileName :type String))
  (bind _returnvalue (Game|GetPlayerController 0))
  ;[1 1 1] Replay시작버튼을 누르고 Replay모드로 전환하는코드
  (Widget|RemovefromParent (Variables|Default|GetRecordNameSettingUI))
  (bind _aspath_tracing_recording_game_instance (Utilities|Casting|CastToPathTracingRecordingGameInstance (Game|GetGameInstance)))
  (Class|PathTracingRecordingGameInstance|StartRecording _aspath_tracing_recording_game_instance ReplayFileName)
  (Input|SetInputModeGameandUI _returnvalue 0 "DoNotLock" true)
  (Variables|/Script/Engine.PlayerController|SetbShowMouseCursor _returnvalue false))

(fn StopRecording
  (bind _returnvalue (Class|RecordingManager|GetIsRecording))
  (if _returnvalue
    (bind _aspath_tracing_recording_game_instance (Utilities|Casting|CastToPathTracingRecordingGameInstance (Game|GetGameInstance)))
    (Class|PathTracingRecordingGameInstance|StopRecording _aspath_tracing_recording_game_instance)
    (Class|RecordingManager|SetIsRecording false)))

(fn ReplayRecording)